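; Prototype weather particle Blueprint that turns Size, Weight and Mass into rain, snow, leaves or fireflies.
; Each Tick compares those values to pick the effect, then derives particle size, alpha, velocity and colour.
; Intensity drives spawn count and random wind, while Radius sets the spawn location, all pushed as parameters to one shared ParticleSystem.
; The construction script displays Intensity on a text render; the Lifetime parameter setter is unconnected.
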(event EventTick
  (params (DeltaSeconds :type Float%20%28single-precision%29))
  (bind _intensity (Variables|Default|GetIntensity))
  (bind _gravity (Variables|Default|GetGravity))
  (bind _particlesystem (Variables|Default|GetParticleSystem))
  (bind _gravity_2 (Variables|Default|GetGravity))
  (bind _mass (Variables|Default|GetMass))
  (bind _radius (Variables|Default|GetRadius))
  (bind _gravity_3 (Variables|Default|GetGravity))
  (bind _mass_2 (Variables|Default|GetMass))
  (bind _gravity_4 (Variables|Default|GetGravity))
  (bind _returnvalue (Math|Float|Absolute(Float) _radius))
  (bind _returnvalue_2 (Math|Float|Absolute(Float) _radius))
  (bind _returnvalue_3 (Math|Float|Absolute(Float) _intensity))
  (bind _returnvalue_4 (* _mass_2 4.0))
  (bind _returnvalue_5 (* _intensity -1.0))
  (bind _returnvalue_6 (Math|Random|RandomFloatinRange _returnvalue _returnvalue_2))
  (bind _returnvalue_7 (Math|Random|RandomFloatinRange _returnvalue_5 _returnvalue_3))
  (bind _returnvalue_8 (Math|Float|Absolute(Float) _returnvalue_6))
  (bind _returnvalue_9 (Math|Float|Absolute(Float) _returnvalue_7))
  (bind _returnvalue_10 (* _returnvalue_6 -1.0))
  (if (> (Variables|Default|GetSize) 0.01)
    (if (> (Variables|Default|GetWeight) 0.01)
      (if (> (Variables|Default|GetMass) 0.01)
        (bind _output_get (Variables|Default|SetLocMin (Math|Vector|MakeVector _returnvalue_10 _returnvalue_10 0.0)))
        (bind _output_get_2 (Variables|Default|SetLocMax (Math|Vector|MakeVector _returnvalue_8 _returnvalue_8 0.0)))
        (Variables|Default|SetInitLoc (Math|Random|RandomPointinBoundingBox _output_get _output_get_2))
        (Variables|Default|SetSpawnCount (* (Math|Float|Absolute(Float) _intensity) (Variables|Default|GetNewVar_0)))
        (Variables|Default|SetWind _returnvalue_9)
        (if (>= _returnvalue_9 1e+01)
          (Variables|Default|SetWind 1e+01))
        ;[1 1 1] Rain
        (if (Math|Boolean|ANDBoolean (> (Variables|Default|GetMass) (Variables|Default|GetSize)) (< (Variables|Default|GetWeight) 0.3) (< (Variables|Default|GetWeight) (Variables|Default|GetSize)))
          (Variables|Default|SetEffect%20Type (Variables|Default|GetRain))
          (if (>= (Variables|Default|GetSize) 2.0)
            (Variables|Default|SetSize 2.0))
          (if (<= (.x (Variables|Default|GetInitSize)) 0.5)
            (Variables|Default|SetInitSize "0.500000,0.500000,0.500000")
            (else
              (Variables|Default|SetInitSize (Math|Vector|MakeVector (* (Variables|Default|GetSize) 0.4) (* (Variables|Default|GetSize) 0.4) (* (Variables|Default|GetSize) 0.4)))))
          (if (>= (* (Variables|Default|GetSize) 0.4) 0.7)
            (Variables|Default|SetInitSize "0.700000,0.700000,0.700000"))
          (Variables|Default|SetAlphaVal (* (Variables|Default|GetMass) 0.2))
          (Variables|Default|SetInitVelo (Math|Vector|MakeVector (* (Math|Random|RandomFloatinRange (* (Variables|Default|GetWind) -1.0) (Math|Float|Absolute(Float) (Variables|Default|GetWind))) 1e+01) (* (Math|Random|RandomFloatinRange (* (Variables|Default|GetWind) -1.0) (Math|Float|Absolute(Float) (Variables|Default|GetWind))) 1e+01) (Math|Random|RandomFloatinRange (* _gravity_2 27.0) (* 3e+01 _gravity_2))))
          (Variables|Default|SetInitColour (Math|Vector|MakeVector 0.0 (* _mass 0.1) (* 0.5 _mass)))
          (Effects|Components|ParticleSystem|SetFloatParameter _particlesystem (Variables|Default|GetAlpha) (Variables|Default|GetAlphaVal) :!label _label)
          (Effects|Components|ParticleSystem|SetVectorParameter _particlesystem (Variables|Default|GetSize_Name) (Variables|Default|GetInitSize))
          (Effects|Components|ParticleSystem|SetVectorParameter _particlesystem (Variables|Default|GetVelocity) (Variables|Default|GetInitVelo))
          (Effects|Components|ParticleSystem|SetVectorParameter _particlesystem (Variables|Default|GetLocation) (Variables|Default|GetInitLoc))
          (Effects|Components|ParticleSystem|SetFloatParameter _particlesystem (Variables|Default|GetSpawn) (Variables|Default|GetSpawnCount))
          (Effects|Components|ParticleSystem|SetVectorParameter _particlesystem (Variables|Default|GetColour) (Variables|Default|GetInitColour))
          (else
            ;[1 1 1] Snow
            (if (Math|Boolean|ANDBoolean (> (Variables|Default|GetSize) (Variables|Default|GetMass)) (< (Variables|Default|GetWeight) 0.3) (< (Variables|Default|GetWeight) (Variables|Default|GetSize)))
              (Variables|Default|SetEffect%20Type (Variables|Default|GetSnow))
              (if (>= (Variables|Default|GetSize) 3.5)
                (Variables|Default|SetSize 3.5))
              (if (<= (.x (Variables|Default|GetInitSize)) 0.5)
                (Variables|Default|SetInitSize "0.500000,0.500000,0.500000")
                (else
                  (Variables|Default|SetInitSize (Math|Vector|MakeVector (* (Variables|Default|GetSize) 0.4) (* (Variables|Default|GetSize) 0.4) (* (Variables|Default|GetSize) 0.4)))))
              (if (>= (* (Variables|Default|GetSize) 0.4) 0.8)
                (Variables|Default|SetInitSize "0.800000,0.800000,0.800000"))
              (Variables|Default|SetAlphaVal (* (Variables|Default|GetMass) 0.5))
              (Variables|Default|SetInitVelo (Math|Vector|MakeVector (* (Math|Random|RandomFloatinRange (* (Variables|Default|GetWind) -1.0) (Math|Float|Absolute(Float) (Variables|Default|GetWind))) 5.0) (* (Math|Random|RandomFloatinRange (* (Variables|Default|GetWind) -1.0) (Math|Float|Absolute(Float) (Variables|Default|GetWind))) 5.0) (Math|Random|RandomFloatinRange (* _gravity_3 3.0) (* 6.0 _gravity_3))))
              (Variables|Default|SetInitColour (Math|Vector|MakeVector _returnvalue_4 _returnvalue_4 _returnvalue_4))
              (goto _label)
              (else
                ;[1 1 1] Leaves
                (if (and (> (Variables|Default|GetWeight) 0.3) (> (Variables|Default|GetSize) (Variables|Default|GetWeight)))
                  (Variables|Default|SetEffect%20Type (Variables|Default|GetLeaves))
                  (if (>= (Variables|Default|GetSize) 4.0)
                    (Variables|Default|SetSize 4.0))
                  (if (<= (.x (Variables|Default|GetInitSize)) 0.7)
                    (Variables|Default|SetInitSize "0.700000,0.700000,0.700000")
                    (else
                      (Variables|Default|SetInitSize (Math|Vector|MakeVector (* (Variables|Default|GetSize) 0.4) (* (Variables|Default|GetSize) 0.4) (* (Variables|Default|GetSize) 0.4)))))
                  (if (>= (* (Variables|Default|GetSize) 0.4) 1.2)
                    (Variables|Default|SetInitSize "1.200000,1.200000,1.200000"))
                  (Variables|Default|SetAlphaVal (* (Variables|Default|GetMass) 1e+01))
                  (Variables|Default|SetInitVelo (Math|Vector|MakeVector (* (Math|Random|RandomFloatinRange (* (Variables|Default|GetWind) -1.0) (Math|Float|Absolute(Float) (Variables|Default|GetWind))) 3.5) (* (Math|Random|RandomFloatinRange (* (Variables|Default|GetWind) -1.0) (Math|Float|Absolute(Float) (Variables|Default|GetWind))) 3.5) (Math|Random|RandomFloatinRange (* _gravity_4 -0.1) (* 3.0 _gravity_4))))
                  (Variables|Default|SetInitColour (Math|Vector|MakeVector (Math|Random|RandomFloatinRange 0.0 (Variables|Default|GetX)) (Variables|Default|GetY) 0.0))
                  (goto _label)
                  (else
                    ;[1 1 1] Fireflies
                    (if (and (> (Variables|Default|GetWeight) 0.3) (> (Variables|Default|GetWeight) (Variables|Default|GetSize)))
                      (Variables|Default|SetEffect%20Type (Variables|Default|GetFireflies))
                      (if (>= (Variables|Default|GetSize) 4.0)
                        (Variables|Default|SetSize 4.0))
                      (if (<= (.x (Variables|Default|GetInitSize)) 0.4)
                        (Variables|Default|SetInitSize "0.400000,0.400000,0.400000")
                        (else
                          (Variables|Default|SetInitSize (Math|Vector|MakeVector (* (Variables|Default|GetSize) 0.4) (* (Variables|Default|GetSize) 0.4) (* (Variables|Default|GetSize) 0.4)))))
                      (if (>= (* (Variables|Default|GetSize) 0.4) 0.6)
                        (Variables|Default|SetInitSize "0.600000,0.600000,0.600000"))
                      (Variables|Default|SetAlphaVal (* (Variables|Default|GetMass) 1e+01))
                      (Variables|Default|SetInitVelo (Math|Vector|MakeVector (* (Math|Random|RandomFloatinRange (* (Variables|Default|GetWind) -1.0) (Math|Float|Absolute(Float) (Variables|Default|GetWind))) (Variables|Default|GetNewVar_0)) (* (Math|Random|RandomFloatinRange (* (Variables|Default|GetWind) -1.0) (Math|Float|Absolute(Float) (Variables|Default|GetWind))) (Variables|Default|GetNewVar_0)) (Math|Random|RandomFloatinRange (* _gravity -0.1) (* -1.0 _gravity))))
                      (Variables|Default|SetInitColour (Math|Vector|MakeVector (Variables|Default|GetFF-Xcol) (Variables|Default|GetZ) 0.0))
                      (goto _label))))))))))))

(event EventBeginPlay
  (Variables|Default|SetWorking? "No"))

(fn ConstructionScript
  (Rendering|Components|TextRender|SetText (Variables|Default|GetTextRenderAA) (Utilities|Text|ToText(Float) (Variables|Default|GetIntensity) "HalfToEven")))