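; Prototype weather particle Blueprint that picks Rain, Snow, Leaves or Fireflies from RGB colour thresholds.
; Each Tick it derives randomized spawn location, wind and velocity, plus size, alpha, spawn count and lifetime, from Intensity, Radius and effect type.
; Particle parameter setters and save-slot preset loading exist but are disconnected, so computed values never reach particles and Enter only prints "LOADED".
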(event EventTick
  (params (DeltaSeconds :type Float%20%28single-precision%29))
  (bind _intensity (Variables|Default|GetIntensity))
  (bind _gravity (Variables|Default|GetGravity))
  (bind _gravity_2 (Variables|Default|GetGravity))
  (bind _radius (Variables|Default|GetRadius))
  (bind _gravity_3 (Variables|Default|GetGravity))
  (bind _gravity_4 (Variables|Default|GetGravity))
  (bind _returnvalue (Math|Float|Absolute(Float) _radius))
  (bind _returnvalue_2 (Math|Float|Absolute(Float) _radius))
  (bind _returnvalue_3 (Math|Float|Absolute(Float) _intensity))
  (bind _returnvalue_4 (* _intensity -1.0))
  (bind _returnvalue_5 (Math|Random|RandomFloatinRange _returnvalue _returnvalue_2))
  (bind _returnvalue_6 (Math|Random|RandomFloatinRange _returnvalue_4 _returnvalue_3))
  (bind _returnvalue_7 (Math|Float|Absolute(Float) _returnvalue_5))
  (bind _returnvalue_8 (Math|Float|Absolute(Float) _returnvalue_6))
  (bind _returnvalue_9 (* _returnvalue_5 -1.0))
  (bind _output_get (Variables|Default|SetLocMin (Math|Vector|MakeVector _returnvalue_9 _returnvalue_9 0.0)))
  (bind _output_get_2 (Variables|Default|SetLocMax (Math|Vector|MakeVector _returnvalue_7 _returnvalue_7 0.0)))
  (Variables|Default|SetInitLoc (Math|Random|RandomPointinBoundingBox _output_get _output_get_2))
  (Variables|Default|SetSize _intensity)
  (Variables|Default|SetWeight _intensity)
  (Variables|Default|SetMass _intensity)
  (Variables|Default|SetSpawnCount (* (Math|Float|Absolute(Float) _intensity) (Variables|Default|GetNewVar_0)))
  (Variables|Default|SetWind _returnvalue_8)
  (if (>= _returnvalue_8 8.0)
    (Variables|Default|SetWind 1e+01))
  ;[1 1 1] Rain
  (if (and (> (Variables|Default|GetInitColZ) (Variables|Default|GetInitColY)) (< (Variables|Default|GetInitColX) 0.15))
    (Variables|Default|SetEffect%20Type (Variables|Default|GetRain))
    (if (> (Variables|Default|GetRadius) 2e+02)
      (Variables|Default|SetSpawnCount (* (Variables|Default|GetSpawnCount) 2.5)))
    (if (>= (Variables|Default|GetSize) 2.0)
      (Variables|Default|SetSize 2.0))
    (if (<= (.x (Variables|Default|GetInitSize)) 0.5)
      (Variables|Default|SetInitSize "0.500000,0.500000,0.500000")
      (else
        (Variables|Default|SetInitSize (Math|Vector|MakeVector (* (Variables|Default|GetSize) 0.4) (* (Variables|Default|GetSize) 0.4) (* (Variables|Default|GetSize) 0.4)))))
    (if (>= (* (Variables|Default|GetSize) 0.4) 0.7)
      (Variables|Default|SetInitSize "0.700000,0.700000,0.700000"))
    (Variables|Default|SetAlphaVal (* (Variables|Default|GetMass) 0.2))
    (Variables|Default|SetInitVelo (Math|Vector|MakeVector (Math|Random|RandomFloatinRange (* (* (Variables|Default|GetWind) -1.0) 1e+01) (* (Math|Float|Absolute(Float) (Variables|Default|GetWind)) 1e+01)) (Math|Random|RandomFloatinRange (* (* (Variables|Default|GetWind) -1.0) 1e+01) (* (Math|Float|Absolute(Float) (Variables|Default|GetWind)) 1e+01)) (Math|Random|RandomFloatinRange (* _gravity_2 27.0) (* 3e+01 _gravity_2))))
    (Variables|Default|SetInitColour (Math|Vector|MakeVector (Variables|Default|GetInitColX) (Variables|Default|GetInitColY) (Variables|Default|GetInitColZ)))
    (Variables|Default|SetLifetime 2.0)
    (else
      ;[1 1 1] Snow
      (if (Math|Boolean|ANDBoolean (> (Variables|Default|GetInitColZ) 0.4) (> (Variables|Default|GetInitColX) 0.4) (> (Variables|Default|GetInitColY) 0.4))
        (Variables|Default|SetEffect%20Type (Variables|Default|GetSnow))
        (if (> (Variables|Default|GetRadius) 2e+02)
          (Variables|Default|SetSpawnCount (* (Variables|Default|GetSpawnCount) 2.0)))
        (if (>= (Variables|Default|GetSize) 3.5)
          (Variables|Default|SetSize 3.5))
        (if (<= (.x (Variables|Default|GetInitSize)) 0.5)
          (Variables|Default|SetInitSize "0.500000,0.500000,0.500000")
          (else
            (Variables|Default|SetInitSize (Math|Vector|MakeVector (* (Variables|Default|GetSize) 0.4) (* (Variables|Default|GetSize) 0.4) (* (Variables|Default|GetSize) 0.4)))))
        (if (>= (* (Variables|Default|GetSize) 0.4) 0.8)
          (Variables|Default|SetInitSize "0.800000,0.800000,0.800000"))
        (Variables|Default|SetAlphaVal (* (Variables|Default|GetMass) 0.5))
        (Variables|Default|SetInitVelo (Math|Vector|MakeVector (* (Math|Random|RandomFloatinRange (* (Variables|Default|GetWind) -1.0) (Math|Float|Absolute(Float) (Variables|Default|GetWind))) 5.0) (* (Math|Random|RandomFloatinRange (* (Variables|Default|GetWind) -1.0) (Math|Float|Absolute(Float) (Variables|Default|GetWind))) 5.0) (Math|Random|RandomFloatinRange (* _gravity_3 3.0) (* 6.0 _gravity_3))))
        (Variables|Default|SetInitColour (Math|Vector|MakeVector (Variables|Default|GetInitColX) (Variables|Default|GetInitColY) (Variables|Default|GetInitColZ)))
        (if (> (Variables|Default|GetRadius) 2e+02)
          (Variables|Default|SetLifetime 2.0)
          (else
            (Variables|Default|SetLifetime 3.0)))
        (else
          ;[1 1 1] Leaves
          (if (and (> (Variables|Default|GetInitColY) (Variables|Default|GetInitColX)) (< (Variables|Default|GetInitColZ) 0.15))
            (Variables|Default|SetEffect%20Type (Variables|Default|GetLeaves))
            (Variables|Default|SetSpawnCount (/ (Variables|Default|GetSpawnCount) 4.0))
            (if (>= (Variables|Default|GetSize) 3.5)
              (Variables|Default|SetSize 3.5))
            (if (<= (.x (Variables|Default|GetInitSize)) 0.7)
              (Variables|Default|SetInitSize "0.700000,0.700000,0.700000")
              (else
                (Variables|Default|SetInitSize (Math|Vector|MakeVector (* (Variables|Default|GetSize) 0.4) (* (Variables|Default|GetSize) 0.4) (* (Variables|Default|GetSize) 0.4)))))
            (if (>= (* (Variables|Default|GetSize) 0.4) 1.2)
              (Variables|Default|SetInitSize "1.200000,1.200000,1.200000"))
            (Variables|Default|SetAlphaVal (* (Variables|Default|GetMass) 1e+01))
            (Variables|Default|SetInitVelo (Math|Vector|MakeVector (* (Math|Random|RandomFloatinRange (* (Variables|Default|GetWind) -1.0) (Math|Float|Absolute(Float) (Variables|Default|GetWind))) 3.5) (* (Math|Random|RandomFloatinRange (* (Variables|Default|GetWind) -1.0) (Math|Float|Absolute(Float) (Variables|Default|GetWind))) 3.5) (Math|Random|RandomFloatinRange (* _gravity_4 -0.1) (* 3.0 _gravity_4))))
            (Variables|Default|SetInitColour (Math|Vector|MakeVector (Variables|Default|GetInitColX) (Variables|Default|GetInitColY) (Variables|Default|GetInitColZ)))
            (Variables|Default|SetLifetime 4.0)
            (else
              ;[1 1 1] Fireflies
              (if (and (> (Variables|Default|GetInitColX) (Variables|Default|GetInitColY)) (< (Variables|Default|GetInitColZ) 0.15))
                (Variables|Default|SetEffect%20Type (Variables|Default|GetFireflies))
                (Variables|Default|SetSpawnCount (/ (Variables|Default|GetSpawnCount) 5.0))
                (if (>= (Variables|Default|GetSize) 4.0)
                  (Variables|Default|SetSize 4.0))
                (if (<= (.x (Variables|Default|GetInitSize)) 0.4)
                  (Variables|Default|SetInitSize "0.400000,0.400000,0.400000")
                  (else
                    (Variables|Default|SetInitSize (Math|Vector|MakeVector (* (Variables|Default|GetSize) 0.4) (* (Variables|Default|GetSize) 0.4) (* (Variables|Default|GetSize) 0.4)))))
                (if (>= (* (Variables|Default|GetSize) 0.4) 0.6)
                  (Variables|Default|SetInitSize "0.600000,0.600000,0.600000"))
                (Variables|Default|SetAlphaVal (* (Variables|Default|GetMass) 1e+01))
                (Variables|Default|SetInitVelo (Math|Vector|MakeVector (* (Math|Random|RandomFloatinRange (* (Variables|Default|GetWind) -1.0) (Math|Float|Absolute(Float) (Variables|Default|GetWind))) 1.5) (* (Math|Random|RandomFloatinRange (* (Variables|Default|GetWind) -1.0) (Math|Float|Absolute(Float) (Variables|Default|GetWind))) 1.5) (Math|Random|RandomFloatinRange (* _gravity -0.1) (* -1.0 _gravity))))
                (Variables|Default|SetInitColour (Math|Vector|MakeVector (Variables|Default|GetInitColX) (Variables|Default|GetInitColY) (Variables|Default|GetInitColZ)))
                (Variables|Default|SetLifetime 5.5)))))))))

(event EventBeginPlay
  (Variables|Default|SetWorking? "No"))

(event Input|KeyboardEvents|Enter
  (params (Key :type Key%20Structure))
  (:Pressed
    (Development|PrintString "LOADED")))

(fn ConstructionScript
  (Rendering|Components|TextRender|SetText (Variables|Default|GetTextRenderAA) (Utilities|Text|ToText(Float) (Variables|Default|GetIntensity) "HalfToEven")))

(fn LoadandSetSavedVar's
  (bind _savegame_ref (Variables|Default|GetSaveGame_Ref))
  (Variables|Default|SetIntensity (Variables|/Game/ProtoStuf/Save_Load/CTP_SaveParams.CTP_SaveParams_C|GetSavedIntensity _savegame_ref))
  (Variables|Default|SetRadius (Variables|/Game/ProtoStuf/Save_Load/CTP_SaveParams.CTP_SaveParams_C|GetSavedRadius _savegame_ref))
  (Variables|Default|SetInitColour (Variables|/Game/ProtoStuf/Save_Load/CTP_SaveParams.CTP_SaveParams_C|GetSavedColour _savegame_ref))
  (Development|PrintString "Loaded Save"))

(fn LoadPreset
  (bind _returnvalue (SaveGame|LoadGamefromSlot (Variables|Default|GetTestSave)))
  (bind _asctp_save_params (Utilities|Casting|CastToCTP_SaveParams _returnvalue))
  (Variables|Default|SetSaveGame_Ref _asctp_save_params)
  (CallFunction|LoadandSetSavedVar's))